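; spawnLogs_bp is a spawner actor that periodically creates moving Log_BP actors at its own transform.
; It spawns one log on BeginPlay, then Tick drives a Delay of LogSpawnTime that gates each further spawn, acting as a repeating timer.
; Each log receives the spawner's LogSpeed and a LifeSpan of ten spawn intervals, which bounds how many logs exist at once.
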(event EventBeginPlay
  (Game|SpawnActorfromClass "/Game/logs/Log_BP.Log_BP_C" (Transformation|GetActorTransform self) "Undefined" "MultiplyWithRoot" 0 (Variables|Default|GetLogSpeed) (* (Variables|Default|GetlogSpawnTime) 1e+01) 0))

(event Collision|EventActorBeginOverlap
  (params (OtherActor :type Actor%20Object%20Reference)))

(event EventTick
  (params (DeltaSeconds :type Float%20%28single-precision%29))
  (Utilities|FlowControl|Delay (Variables|Default|GetlogSpawnTime))
  (Game|SpawnActorfromClass "/Game/logs/Log_BP.Log_BP_C" (Transformation|GetActorTransform self) "Undefined" "MultiplyWithRoot" 0 (Variables|Default|GetLogSpeed) (* (Variables|Default|GetlogSpawnTime) 1e+01) 0))

(fn ConstructionScript)